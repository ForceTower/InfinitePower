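; Player character for an InfiniteBox game that moves along Y and switches gravity between down, up and two sideways directions with key presses, recoloring its cube.
; Tick applies custom gravity as capsule acceleration, and Jump pushes against it or kicks off touched walls when airborne.
; Side overlap components set the wall and Landed flags for jumping and movement blocking.
; Horizontal input offsets the actor only under vertical gravity.
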(event `InputAction|Jump`
  (params (Key :type "Key Structure"))
  (bind _capsulecomponent (`self.CapsuleComponent`))
  (bind _capsulecomponent_2 (`self.CapsuleComponent`))
  (bind _gravity (`self.Gravity`))
  (bind _returnvalue (select `bool` (`self.RightWall`) :`false` (select `bool` (`self.LeftWall`) :`true` 21000.0 :!type "Float (single-precision)") :`true` -21000.0))
  (bind _returnvalue_2 (!= _returnvalue 0.0))
  (:`Pressed`
    (if (`self.Landed`)
      (switch `int` _gravity
        (:`0`
          (`PrimitiveComponent.AddForce` _capsulecomponent_2 (0.0 0.0 21000.0) "None" true))
        (:`1`
          (`PrimitiveComponent.AddForce` _capsulecomponent_2 (0.0 0.0 -21000.0) "None" true))
        (:`2`
          (`PrimitiveComponent.AddForce` _capsulecomponent_2 (0.0 -21000.0 0.0) "None" true))
        (:`3`
          (`PrimitiveComponent.AddForce` _capsulecomponent_2 (0.0 21000.0 0.0) "None" true)))
      (else
        (switch `int` _gravity
          (:`0`
            (if _returnvalue_2
              (`PrimitiveComponent.AddForce` _capsulecomponent (`KismetMathLibrary.MakeVector` 0.0 _returnvalue 21000.0) "None" true)))
          (:`1`
            (if _returnvalue_2
              (`PrimitiveComponent.AddForce` _capsulecomponent (`KismetMathLibrary.MakeVector` 0.0 _returnvalue -21000.0) "None" true)))
          (:`2`
            (if _returnvalue_2
              (`PrimitiveComponent.AddForce` _capsulecomponent (`KismetMathLibrary.MakeVector` 0.0 -21000.0 _returnvalue) "None" true)))
          (:`3`
            (if _returnvalue_2
              (`PrimitiveComponent.AddForce` _capsulecomponent (`KismetMathLibrary.MakeVector` 0.0 21000.0 _returnvalue) "None" true))))))))

(event `self.ReceiveTick`
  (params (DeltaSeconds :type "Float (single-precision)"))
  (`|ExecutionSequence`
    (:`then_0`
      (switch `int` (`self.Gravity`)
        (:`0`
          (`PrimitiveComponent.AddForce` (`self.CapsuleComponent`) (0.0 0.0 -980.0) "None" true))
        (:`1`
          (`PrimitiveComponent.AddForce` (`self.CapsuleComponent`) (0.0 0.0 980.0) "None" true))
        (:`2`
          (`PrimitiveComponent.AddForce` (`self.CapsuleComponent`) (0.0 980.0 0.0) "None" true))
        (:`3`
          (`PrimitiveComponent.AddForce` (`self.CapsuleComponent`) (0.0 -980.0 0.0) "None" true))))))

(event `InputAxis|Move Horizontal`
  (params (AxisValue :type "Float (single-precision)"))
  (bind _gravity (`self.Gravity`))
  (if (and (or (== _gravity 0) (== _gravity 1)) (not (or (and (`self.RightWall`) (> AxisValue 0.0)) (and (`self.LeftWall`) (< AxisValue 0.0)))))
    (`self.K2_AddActorLocalOffset` (`KismetMathLibrary.MakeVector` 0.0 (* (* (stale `self.ReceiveTick` DeltaSeconds) AxisValue) 420.0)))))

(event `Key|Up`
  (params (Key :type "Key Structure"))
  (:`Pressed`
    (set `self.Gravity` 1)
    (`MaterialInstanceDynamic.SetVectorParameterValue` (`self.Material`) "Color" (struct :`R` 0.011136 :`G` 1.0 :`A` 1.0))
    (`KismetSystemLibrary.PrintString` "Changed Gravity" :!label _label)))

(event `Key|Down`
  (params (Key :type "Key Structure"))
  (:`Pressed`
    (set `self.Gravity` 0)
    (`MaterialInstanceDynamic.SetVectorParameterValue` (`self.Material`) "Color" (struct :`G` 0.582093 :`B` 1.0 :`A` 1.0))
    (goto _label)))

(event `Key|Left`
  (params (Key :type "Key Structure"))
  (:`Pressed`
    (set `self.Gravity` 2)
    (`MaterialInstanceDynamic.SetVectorParameterValue` (`self.Material`) "Color" (struct :`R` 0.946525 :`G` 1.0 :`A` 1.0))
    (goto _label)))

(event `Key|Right`
  (params (Key :type "Key Structure"))
  (:`Pressed`
    (set `self.Gravity` 3)
    (`MaterialInstanceDynamic.SetVectorParameterValue` (`self.Material`) "Color" (struct :`R` 1.0 :`B` 0.007639 :`A` 1.0))
    (goto _label)))

(event `self.Right.OnComponentBeginOverlap`
  (params (OverlappedComponent :type "PrimitiveComponent Object Reference") (OtherActor :type "Actor Object Reference") (OtherComp :type "PrimitiveComponent Object Reference") (OtherBodyIndex :type Integer) (bFromSweep :type Boolean) (SweepResult :type "HitResult Structure (by ref)"))
  (if (!= OtherActor self)
    (`|ExecutionSequence`
      (:`then_0`
        (set `self.RightWall` true))
      (:`then_1`
        (set `self.Landed` (== (`self.Gravity`) 1))))))

(event `self.Right.OnComponentEndOverlap`
  (params (OverlappedComponent :type "PrimitiveComponent Object Reference") (OtherActor :type "Actor Object Reference") (OtherComp :type "PrimitiveComponent Object Reference") (OtherBodyIndex :type Integer))
  (if (!= OtherActor self)
    (`|ExecutionSequence`
      (:`then_0`
        (set `self.RightWall` false))
      (:`then_1`
        (set `self.Landed` (not (== (`self.Gravity`) 1)))))))

(event `self.Left.OnComponentBeginOverlap`
  (params (OverlappedComponent :type "PrimitiveComponent Object Reference") (OtherActor :type "Actor Object Reference") (OtherComp :type "PrimitiveComponent Object Reference") (OtherBodyIndex :type Integer) (bFromSweep :type Boolean) (SweepResult :type "HitResult Structure (by ref)"))
  (if (!= OtherActor self)
    (set `self.LeftWall` true)))

(event `self.Left.OnComponentEndOverlap`
  (params (OverlappedComponent :type "PrimitiveComponent Object Reference") (OtherActor :type "Actor Object Reference") (OtherComp :type "PrimitiveComponent Object Reference") (OtherBodyIndex :type Integer))
  (if (!= OtherActor self)
    (set `self.LeftWall` false)))

(event `self.Down.OnComponentBeginOverlap`
  (params (OverlappedComponent :type "PrimitiveComponent Object Reference") (OtherActor :type "Actor Object Reference") (OtherComp :type "PrimitiveComponent Object Reference") (OtherBodyIndex :type Integer) (bFromSweep :type Boolean) (SweepResult :type "HitResult Structure (by ref)"))
  (if (!= OtherActor self)
    (set `self.Landed` (== (`self.Gravity`) 0))))

(event `self.Down.OnComponentEndOverlap`
  (params (OverlappedComponent :type "PrimitiveComponent Object Reference") (OtherActor :type "Actor Object Reference") (OtherComp :type "PrimitiveComponent Object Reference") (OtherBodyIndex :type Integer))
  (if (!= OtherActor self)
    (set `self.Landed` (not (== (`self.Gravity`) 0)))))

(event `self.Up.OnComponentBeginOverlap`
  (params (OverlappedComponent :type "PrimitiveComponent Object Reference") (OtherActor :type "Actor Object Reference") (OtherComp :type "PrimitiveComponent Object Reference") (OtherBodyIndex :type Integer) (bFromSweep :type Boolean) (SweepResult :type "HitResult Structure (by ref)"))
  (if (!= OtherActor self)
    (set `self.Landed` (== (`self.Gravity`) 1))))

(event `self.Up.OnComponentEndOverlap`
  (params (OverlappedComponent :type "PrimitiveComponent Object Reference") (OtherActor :type "Actor Object Reference") (OtherComp :type "PrimitiveComponent Object Reference") (OtherBodyIndex :type Integer))
  (if (!= self OtherActor)
    (set `self.Landed` (not (== (`self.Gravity`) 1)))))

(fn `UserConstructionScript`
  (bind _returnvalue (`PrimitiveComponent.CreateDynamicMaterialInstance` (`self.Cube`) 0 null))
  (set `self.Material` _returnvalue))